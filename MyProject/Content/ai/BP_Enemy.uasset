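; Enemy AI actor Blueprint that supplies patrol destinations from the level's TargetPoints.
; On BeginPlay it gathers every TargetPoint actor in the level into its PatrolPoints array.
; GetNextPatrolPoint returns the current point's location, then advances the index and wraps to the first after the last.
; The Blueprint itself contains no movement logic.
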(event EventBeginPlay
  (bind _outactors (Actor|GetAllActorsOfClass "/Script/Engine.TargetPoint"))
  (Variables|Default|SetPatrol%20Points _outactors))

(event Collision|EventActorBeginOverlap
  (params (OtherActor :type Actor%20Object%20Reference)))

(event EventTick
  (params (DeltaSeconds :type Float%20%28single-precision%29)))

(fn ConstructionScript)

(fn GetNextPatrolPoint
  (LocalVariables|Setpaatrol%20point%20loc (Transformation|GetActorLocation (Utilities|Array|Get(acopy) (Variables|Default|GetPatrol%20Points) (Variables|Default|GetCurrent%20patrol%20index))))
  (bind _result (Math|Integer|IncrementInt (Variables|Default|GetCurrent%20patrol%20index))
    (:%20%20
      (if (>= _result (Utilities|Array|Length (Variables|Default|GetPatrol%20Points)))
        (Variables|Default|SetCurrent%20patrol%20index 0))
      (return (LocalVariables|Getpaatrol%20point%20loc)))))