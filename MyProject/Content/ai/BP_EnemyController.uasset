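; BP_EnemyController is the AI controller for BP_Enemy, switching it between patrolling and chasing perceived actors.
; After a one-second startup delay, it caches the pawn and loops AIMoveTo through the pawn's patrol points, advancing only on success.
; A successful perception stimulus stops movement and sends the pawn after the sensed actor.
; An unsuccessful stimulus clears the target and restarts the patrol from the current point.
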(event OnTargetPerceptionUpdated(AIPerception)
  (params (Actor :type Actor%20Object%20Reference) (Stimulus :type AI%20Stimulus%20Structure))
  (if (.bsuccessfullysensed Stimulus)
    (bind _output_get (Variables|Default|SetTarget%20actor Actor))
    (AI|Navigation|StopMovement)
    (AI|AIMoveTo (Variables|Default|GetPawn%20Ref) "0, 0, 0" _output_get 5.0 false)
    (else
      (Variables|Default|SetTarget%20actor 0)
      (CallFunction|Patrol))))

(event Custom|patrol
  (bind _pawn_ref (Variables|Default|GetPawn%20Ref))
  (AI|AIMoveTo (Variables|Default|GetPawn%20Ref) (Transformation|GetActorLocation (Utilities|Array|Get(acopy) (Variables|/Game/ai/BP_Enemy.BP_Enemy_C|GetPatrol%20Points _pawn_ref) (Variables|/Game/ai/BP_Enemy.BP_Enemy_C|GetCurrent%20patrol%20index _pawn_ref))) 0 5.0 false
    (:OnSuccess
      (Default|GetNextPatrolPoint (Variables|Default|GetPawn%20Ref))
      (CallFunction|Patrol))))

(event EventBeginPlay
  (Utilities|FlowControl|Delay 1.0)
  (bind _asbp_enemy (Utilities|Casting|CastToBP_Enemy (Pawn|GetControlledPawn)))
  (Variables|Default|SetPawn%20Ref _asbp_enemy)
  (CallFunction|Patrol))

(fn ConstructionScript)