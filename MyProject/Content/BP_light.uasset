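; BP_light is an actor that acts as a light switch, controlling a referenced Lightbulb actor.
; When a BP_FirstPersonCharacter overlaps it, it hides the bulb, sets the character's Lightoff flag and enables player input on itself.
; The F key then drives a FlipFlop that alternately shows and hides the bulb, updating Lightoff to match.
; No end-overlap logic disables input, so F stays bound after the character leaves.
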(event Collision|EventActorBeginOverlap
  (params (OtherActor :type Actor%20Object%20Reference))
  (bind _asbp_first_person_character (Utilities|Casting|CastToBP_FirstPersonCharacter OtherActor))
  (Variables|/Game/FirstPerson/Blueprints/BP_FirstPersonCharacter.BP_FirstPersonCharacter_C|Setlightoff? _asbp_first_person_character true)
  (Rendering|SetActorHiddenInGame (Variables|Default|GetLightbulb) true)
  (Input|EnableInput (Game|GetPlayerController 0)))

(event Input|KeyboardEvents|F
  (params (Key :type Key%20Structure :default "None"))
  (bind _lightbulb (Variables|Default|GetLightbulb))
  (:Pressed
    (Utilities|FlowControl|FlipFlop
      (:A
        (Rendering|SetActorHiddenInGame _lightbulb false)
        (Variables|/Game/FirstPerson/Blueprints/BP_FirstPersonCharacter.BP_FirstPersonCharacter_C|Setlightoff? (stale Collision|EventActorBeginOverlap _asbp_first_person_character) false))
      (:B
        (Rendering|SetActorHiddenInGame _lightbulb true)
        (Variables|/Game/FirstPerson/Blueprints/BP_FirstPersonCharacter.BP_FirstPersonCharacter_C|Setlightoff? (stale Collision|EventActorBeginOverlap _asbp_first_person_character) true)))))

(fn ConstructionScript)