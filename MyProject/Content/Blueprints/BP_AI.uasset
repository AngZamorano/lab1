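; BP_AI is an enemy pawn that chases the player and leaves a key behind when it is removed.
; Tick issues AIMoveTo toward player pawn 0 every frame, and both hit and overlap events call Died on BP_FirstPersonCharacter.
; Six seconds after BeginPlay it calls Kill, which spawns BP_Key at the mesh location and destroys the actor.
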(event Custom|Kill
  (Game|SpawnActorfromClass "/Game/Blueprints/BP_Key.BP_Key_C" (Math|Conversions|ToTransform(Vector) (Transformation|GetWorldLocation (Variables|Character|GetMesh))) "Undefined" "MultiplyWithRoot" 0 0)
  (Actor|DestroyActor))

(event EventBeginPlay
  (Utilities|FlowControl|Delay 6.0)
  (CallFunction|Kill))

(event Collision|EventActorBeginOverlap
  (params (OtherActor :type Actor%20Object%20Reference))
  (bind _asbp_first_person_character (Utilities|Casting|CastToBP_FirstPersonCharacter (stale Collision|EventHit Other)))
  (Default|Died _asbp_first_person_character))

(event EventTick
  (params (DeltaSeconds :type Float%20%28single-precision%29))
  (AI|AIMoveTo self "0, 0, 0" (Game|Player|GetPlayerPawn 0) 5.0 false))

(event Collision|EventHit
  (params (MyComp :type Primitive%20Component%20Object%20Reference) (Other :type Actor%20Object%20Reference) (OtherComp :type Primitive%20Component%20Object%20Reference) (bSelfMoved :type Boolean) (HitLocation :type Vector :default "0, 0, 0") (HitNormal :type Vector :default "0, 0, 0") (NormalImpulse :type Vector :default "0, 0, 0") (Hit :type Hit%20Result%20Structure%20%28by%20ref%29))
  (bind _asbp_first_person_character (Utilities|Casting|CastToBP_FirstPersonCharacter Other))
  (Default|Died _asbp_first_person_character))

(fn ConstructionScript)