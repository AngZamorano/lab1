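; BP_Animal is an animal actor that announces its sound and moves steadily through the world.
; On BeginPlay, MakeSound prints a string built from its Species and Sound variables; no audio plays.
; Each Tick passes MoveSpeed scaled by delta time to Move, which offsets the Cube component equally along world X and Y, with sweep enabled for collision.
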(event Custom|MakeSound
  (params (sound :type String) (Species :type String))
  (Development|PrintString (Utilities|String|Append Species " says " sound)))

(event Custom|Move
  (params (speed :type Float%20%28double-precision%29))
  (Transformation|AddWorldOffset (Variables|Default|GetCube) (Math|Vector|MakeVector speed speed 0.0) true false))

(event EventBeginPlay
  (CallFunction|MakeSound (Variables|Default|GetSound) (Variables|Default|GetSpecies)))

(event Collision|EventActorBeginOverlap
  (params (OtherActor :type Actor%20Object%20Reference)))

(event EventTick
  (params (DeltaSeconds :type Float%20%28single-precision%29))
  (CallFunction|Move (* DeltaSeconds (Variables|Default|GetMoveSpeed))))

(fn ConstructionScript)