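; BP_Eagle is an eagle actor whose Cube component moves along the world Z axis while it runs.
; Tick offsets the Cube by MoveSpeed scaled by delta time, for frame-rate-independent motion.
; After calling its parent, BeginPlay waits through a fixed delay, then calls the custom ISee event, which prints the Food variable.
; The overlap event is disabled, and the construction script only calls its parent.
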(event Custom|I%20see
  (Development|PrintString (Variables|Default|Getfood)))

(event EventBeginPlay
  (|CallParentFunction)
  (Utilities|FlowControl|Delay 2e+01)
  (CallFunction|ISee))

(event Collision|EventActorBeginOverlap
  (params (OtherActor :type Actor%20Object%20Reference))
  (|CallParentFunction OtherActor) ; This node is disabled and will not be called.\nDrag off pins to build functionality.
)

(event EventTick
  (params (DeltaSeconds :type Float%20%28single-precision%29))
  (|CallParentFunction DeltaSeconds)
  (Transformation|AddWorldOffset (Variables|Default|GetCube) (Math|Vector|MakeVector 0.0 0.0 (* DeltaSeconds (Variables|Default|GetMoveSpeed))) false false))

(fn ConstructionScript
  (|CallParentFunction))