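; BP_NPC is an NPC Blueprint that shows a dialog line, then hands the dialog widget over to the player character.
; Dialog creates WBP_Dialog only when no valid reference exists, stores it, adds it to the viewport, shows its blur and fills in the Talk text.
; Finish hides the blur, reveals the widget's Timer and passes the widget to BP_FirstPersonCharacter through GetWidget.
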(event EventBeginPlay)

(event Collision|EventActorBeginOverlap
  (params (OtherActor :type Actor%20Object%20Reference)))

(event EventTick
  (params (DeltaSeconds :type Float%20%28single-precision%29)))

(event EventDialog
  (Variables|Default|GetUI%20Ref
    (:then)
    (:else
      (bind _returnvalue (UserInterface|CreateWidget "/Game/Blueprints/WBP_Dialog.WBP_Dialog_C" (Game|GetPlayerController 0)))
      (bind _output_get (Variables|Default|SetUI%20Ref _returnvalue))
      (UserInterface|Viewport|AddtoViewport _output_get 0)
      (Widget|SetVisibility (Variables|/Game/Blueprints/WBP_Dialog.WBP_Dialog_C|Getblur _output_get) "Visible")
      (Rendering|Components|TextRender|SetText (Variables|/Game/Blueprints/WBP_Dialog.WBP_Dialog_C|Gettalk _output_get) (Utilities|Text|ToText(String) (Variables|Default|GetTalk))))))

(event EventFinish
  (bind _ui_ref (Variables|Default|GetUI%20Ref)
    (:then
      (Widget|SetVisibility (Variables|/Game/Blueprints/WBP_Dialog.WBP_Dialog_C|Getblur _ui_ref) "Hidden")
      (Widget|SetVisibility (Variables|/Game/Blueprints/WBP_Dialog.WBP_Dialog_C|GetTimer _ui_ref) "Visible")
      (bind _asbp_first_person_character (Utilities|Casting|CastToBP_FirstPersonCharacter (Game|GetPlayerCharacter 0)))
      (Default|GetWidget _asbp_first_person_character (Variables|Default|GetUI%20Ref)))
    (:else)))

(fn ConstructionScript)