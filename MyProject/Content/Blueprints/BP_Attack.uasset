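; BP_Attack is an AI-moved attacker that heads for the level's BP_Tower and can be killed by hits.
; On BeginPlay it finds the tower and runs AI Move To toward it, reissuing the move two seconds after each successful arrival.
; The hit event decrements Health, and Tick polls it, calling ActorDied on the tower and destroying the actor once Health runs out.
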(event Custom|hit
  (Variables|Default|Sethealth (- (Variables|Default|Gethealth) 1)))

(event EventBeginPlay
  (bind _returnvalue (Actor|GetActorOfClass "/Game/Blueprints/BP_Tower.BP_Tower_C"))
  (bind _output_get (Variables|Default|SetTower%20Ref _returnvalue))
  (AI|AIMoveTo self "0, 0, 0" _output_get 5.0 false :!label _label
    (:OnSuccess
      (Utilities|FlowControl|Delay 2.0)
      (goto _label))))

(event EventTick
  (params (DeltaSeconds :type Float%20%28single-precision%29))
  (if (<= (Variables|Default|Gethealth) 0)
    (Default|ActorDied (Variables|Default|GetTower%20Ref))
    (Actor|DestroyActor)))

(fn ConstructionScript)