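; BP_Tower is an automated turret that shoots BP_Attack actors entering its Range component.
; Overlaps append targets to an array, and the actordied event advances the target index without removing entries.
; Tick uses Delays to pace shots: a debug-drawn line trace from the Cylinder to the current target calls Hit and spends ammo.
; An empty tower refills its ammo after a longer delay.
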(event OnComponentBeginOverlap(range)
  (params (OverlappedComponent :type Primitive%20Component%20Object%20Reference) (OtherActor :type Actor%20Object%20Reference) (OtherComp :type Primitive%20Component%20Object%20Reference) (OtherBodyIndex :type Integer) (bFromSweep :type Boolean) (SweepResult :type Hit%20Result%20Structure%20%28by%20ref%29))
  (bind _asbp_attack (Utilities|Casting|CastToBP_Attack OtherActor))
  (Utilities|Array|Add (Variables|Default|GetActors) _asbp_attack))

(event Custom|actor%20died
  (Math|Integer|IncrementInt (Variables|Default|Getcurrent%20index)))

(event Collision|EventActorBeginOverlap
  (params (OtherActor :type Actor%20Object%20Reference)))

(event EventTick
  (params (DeltaSeconds :type Float%20%28single-precision%29))
  (bind _actors (Variables|Default|GetActors))
  (bind _current_index (Variables|Default|Getcurrent%20index))
  (if (> (Variables|Default|GetAmmo) 0)
    (Utilities|FlowControl|Delay 2.0)
    (if (Utilities|Array|IsValidIndex _actors _current_index)
      (if (Utilities|Array|IsNotEmpty _actors)
        (bind (_outhit _returnvalue) (Collision|LineTraceForObjects (Transformation|GetWorldLocation (Variables|Default|GetCylinder)) (Transformation|GetWorldLocation (Variables|/Script/Engine.Character|GetCapsuleComponent (Utilities|Array|Get(acopy) _actors _current_index))) (Utilities|Array|MakeArray "ObjectTypeQuery3") false 0 "Persistent"))
        (if _returnvalue
          (bind _asbp_attack (Utilities|Casting|CastToBP_Attack (.hitactor _outhit)))
          (Default|Hit _asbp_attack)
          (Math|Integer|DecrementInt (Variables|Default|GetAmmo)))))
    (else
      (Utilities|FlowControl|Delay 1e+01)
      (Variables|Default|SetAmmo 10))))

(fn ConstructionScript)