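; BP_Turtle is a minimal turtle Blueprint that periodically prints a TurtleGoesVerySlow debug message, with no movement logic in its graphs.
; Tick calls the parent, then runs a two-second Delay into the Slow event, which does the printing.
; The Delay ignores re-triggers while pending, so it throttles the per-frame Tick to roughly one message every two seconds.
; BeginPlay and overlap events are disabled stubs, and construction only calls the parent.
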(event Custom|slow
  (Development|PrintString (Variables|Default|GetTurtle%20goes%20very%20slow)))

(event EventBeginPlay
  (|CallParentFunction) ; This node is disabled and will not be called.\nDrag off pins to build functionality.
)

(event Collision|EventActorBeginOverlap
  (params (OtherActor :type Actor%20Object%20Reference))
  (|CallParentFunction OtherActor) ; This node is disabled and will not be called.\nDrag off pins to build functionality.
)

(event EventTick
  (params (DeltaSeconds :type Float%20%28single-precision%29))
  (Utilities|FlowControl|Sequence
    (:then_0
      (|CallParentFunction DeltaSeconds))
    (:then_1
      (Utilities|FlowControl|Delay 2.0)
      (CallFunction|Slow))))

(fn ConstructionScript
  (|CallParentFunction))